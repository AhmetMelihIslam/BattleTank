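; Player-controllable tank Blueprint that routes input to movement, camera and weapon logic.
; On BeginPlay it initialises the TankAiminng component with barrel and turret, initialises TankMovement, and hands itself to its HealthBar widget.
; Drive and fire inputs forward to those components, while aim axes rotate the azimuth gimbal (yaw) and spring arm (pitch), scaled by delta time.
; Swap Cam toggles the first- and third-person cameras.
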(event `self.ReceiveBeginPlay`
  (`TankAiminngComponent.Initialise` (`self.TankAiminng`) (`self.Barrel`) (`self.Turret`))
  (`TankMovementComponent.Initialise` (`self.TankMovement`) null null)
  (`self.InitiliseHealthBarWidget`))

(event `InputAxis|AimAzimuth`
  (params (AxisValue :type "Float (single-precision)"))
  ;[1 1 1] Balistics Input Binding
  (`SceneComponent.K2_AddLocalRotation` (`self.Azimult Gimbal`) (`KismetMathLibrary.MakeRotator` 0.0 0.0 (* AxisValue (`GameplayStatics.GetWorldDeltaSeconds`) 100.0)) false false))

(event `InputAxis|Move Forward`
  (params (AxisValue :type "Float (single-precision)"))
  ;[1 1 1] Movement Input Binding
  (`TankMovementComponent.IntendMoveForward` (`self.TankMovement`) AxisValue))

(event `InputAxis|Turn Right`
  (params (AxisValue :type "Float (single-precision)"))
  ;[1 1 1] Movement Input Binding
  (`TankMovementComponent.IntendTurnRight` (`self.TankMovement`) AxisValue))

(event `InputAxis|AimElevation`
  (params (AxisValue :type "Float (single-precision)"))
  ;[1 1 1] Balistics Input Binding
  (`SceneComponent.K2_AddLocalRotation` (`self.SpringArm`) (`KismetMathLibrary.MakeRotator` 0.0 (* AxisValue (`GameplayStatics.GetWorldDeltaSeconds`) 100.0)) false false))

(event `InputAction|Fire`
  (params (Key :type "Key Structure"))
  ;[1 1 1] Balistics Input Binding
  (:`Pressed`
    (`TankAiminngComponent.Fire` (`self.TankAiminng`))))

(event `InputAction|Swap Cam`
  (params (Key :type "Key Structure"))
  ;[1 1 1] Camera Swapping
  (:`Pressed`
    (`ActorComponent.ToggleActive` (`self.1st person`))
    (`ActorComponent.ToggleActive` (`self.3rd person`))))

(fn `InitiliseHealthBarWidget`
  (bind _ashealth_bar (cast `/Game/UI/HealthBar` (`WidgetComponent.GetUserWidgetObject` (`self.HealthBar`))))
  (set `/Game/UI/HealthBar.MyTank` self _ashealth_bar))

(fn `UserConstructionScript`)